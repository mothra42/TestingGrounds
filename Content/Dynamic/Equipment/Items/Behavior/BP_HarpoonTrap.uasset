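; BP_HarpoonTrap is a harpoon trap that fires on any character other than player 0's pawn entering its fire trigger.
; Overlap calls FireTrap and applies heavy damage, then teleports the trapped actor's mesh to CharacterAttachmentPoint and snaps its AttachmentPoint component there.
; A hit on the trap body calls OrientTrapToSurface to align the trap.
; The second trigger box's overlap is empty, and an AttachActorToTrap branch is unwired.
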(event OnComponentBeginOverlap(TrapTriggerBox)
  (params (OverlappedComponent :type Primitive%20Component%20Object%20Reference) (OtherActor :type Actor%20Object%20Reference) (OtherComp :type Primitive%20Component%20Object%20Reference) (OtherBodyIndex :type Integer) (bFromSweep :type Boolean) (SweepResult :type Hit%20Result%20Structure%20%28by%20ref%29)))

(event OnComponentBeginOverlap(FireTriggerBox)
  (params (OverlappedComponent :type Primitive%20Component%20Object%20Reference) (OtherActor :type Actor%20Object%20Reference) (OtherComp :type Primitive%20Component%20Object%20Reference) (OtherBodyIndex :type Integer) (bFromSweep :type Boolean) (SweepResult :type Hit%20Result%20Structure%20%28by%20ref%29))
  (bind _trappedactor (Variables|Default|GetTrappedActor))
  (bind _asbp_character (Utilities|Casting|CastToBP_Character OtherActor))
  (if (not (== _asbp_character (Game|Player|GetPlayerPawn 0)))
    (Class|HarpoonTrap|FireTrap _asbp_character)
    (Game|Damage|ApplyDamage _asbp_character 1e+02 0 0)
    (Utilities|IsValid _trappedactor
      (:Is%20Valid
        (Transformation|SetWorldLocation (Variables|/Script/Engine.Character|GetMesh _trappedactor) (Transformation|GetWorldLocation (Variables|Default|GetCharacterAttachmentPoint)) false true)
        (Transformation|AttachComponentToComponent (Variables|/Script/TestingGrounds.Mannequin|GetAttachmentPoint _trappedactor) (Variables|Default|GetCharacterAttachmentPoint) "None" "SnapToTarget" "KeepRelative" "KeepRelative" false)))))

(event OnComponentHit(TrapBody)
  (params (HitComponent :type Primitive%20Component%20Object%20Reference) (OtherActor :type Actor%20Object%20Reference) (OtherComp :type Primitive%20Component%20Object%20Reference) (NormalImpulse :type Vector :default "0, 0, 0") (Hit :type Hit%20Result%20Structure%20%28by%20ref%29))
  (Class|HarpoonTrap|OrientTraptoSurface Hit))

(fn ConstructionScript)