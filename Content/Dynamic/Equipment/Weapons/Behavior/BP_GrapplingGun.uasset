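; Grappling gun weapon Blueprint that applies force to the player character while the hook is attached.
; BeginPlay caches player 0's character.
; Tick polls the left mouse button directly on the player controller and, while it is held and IsAttached is true, calls ApplyForceToCharacter each frame.
; The attach logic and the force calculation are not defined in these graphs.
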(event EventBeginPlay
  ;[1 1 1] Get Player
  (Variables|Default|SetPlayerCharacter (Game|GetPlayerCharacter 0)))

(event EventTick
  (params (DeltaSeconds :type Float%20%28single-precision%29))
  ;[1 1 1] Apply Force
  (if (Game|Player|IsInputKeyDown (Game|GetPlayerController 0) "LeftMouseButton")
    (if (Variables|Default|GetisAttached)
      (Class|GrapplingGun|ApplyForcetoCharacter))))

(fn ConstructionScript)