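; BP_GrapplingGun is a first-person weapon behaviour Blueprint for a grappling gun that applies force to the player character while attached.
; BeginPlay caches the player character, and Tick calls ApplyForceToCharacter while the left mouse button is held and IsAttached is true.
; Releasing the Fire action clears IsAttached; nothing in this graph sets it.
; An unconnected character-movement AddForce chain with a zero vector never runs.
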(event EventBeginPlay
  (Variables|Default|SetPlayerCharacter (Game|GetPlayerCharacter 0)))

(event EventTick
  (params (DeltaSeconds :type Float%20%28single-precision%29))
  ;[1 1 1] Apply Force
  (if (Game|Player|IsInputKeyDown (Game|GetPlayerController 0) "LeftMouseButton")
    (if (Variables|Default|GetisAttached)
      (Class|GrapplingGun|ApplyForcetoCharacter))))

(event Input|ActionEvents|InputActionFire
  (params (Key :type Key%20Structure :default "None"))
  ;[1 1 1] Set Attached State To False
  (:Released
    (Variables|Default|SetisAttached false)))

(fn ConstructionScript)